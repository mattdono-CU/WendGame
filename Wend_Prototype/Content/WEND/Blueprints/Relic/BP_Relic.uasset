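; BP_Relic is a relic actor that spins and hovers in place, and destroys itself on a Hit event.
; BeginPlay stores the relative start location of the SMRelicCircle mesh.
; Tick rotates that mesh in yaw and moves it vertically, both scaled by delta time, flipping the vertical speed whenever it reaches the offset limit above or below the start height.
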(event EventBeginPlay
  ;[1 1 1] Get Starting Position of Relic
  (Variables|Default|SetStartPosition (Variables|/Script/Engine.SceneComponent|GetRelativeLocation (Variables|Default|GetSM_Relic_Circle))))

(event Collision|EventActorBeginOverlap
  (params (OtherActor :type Actor%20Object%20Reference)))

(event EventTick
  (params (DeltaSeconds :type Float%20%28single-precision%29))
  (bind _startposition (Variables|Default|GetStartPosition))
  (bind _sm_relic_circle (Variables|Default|GetSM_Relic_Circle))
  (bind _offsetmax (Variables|Default|GetOffsetMax))
  (bind _relativelocation (Variables|/Script/Engine.SceneComponent|GetRelativeLocation _sm_relic_circle))
  ;[1 1 1] Relic Hover / Rotation Animation
  (Utilities|FlowControl|Sequence
    (:then_0
      (Transformation|AddLocalRotation (Variables|Default|GetSM_Relic_Circle) (Math|Rotator|MakeRotator 0.0 0.0 (* (Variables|Default|GetRotationPerSecond) DeltaSeconds)) false false))
    (:then_1
      (Utilities|FlowControl|Sequence
        (:then_0
          (if (or (>= (.z _relativelocation) (+ (.z _startposition) _offsetmax)) (<= (.z _relativelocation) (- (.z _startposition) _offsetmax)))
            (Variables|Default|SetOffsetPerSecond (* (Variables|Default|GetOffsetPerSecond) -1.0))))
        (:then_1
          (Transformation|AddWorldOffset (Variables|Default|GetSM_Relic_Circle) (Math|Vector|MakeVector 0.0 0.0 (* DeltaSeconds (Variables|Default|GetOffsetPerSecond))) false false))))))

(event Collision|EventHit
  (params (MyComp :type Primitive%20Component%20Object%20Reference) (Other :type Actor%20Object%20Reference) (OtherComp :type Primitive%20Component%20Object%20Reference) (bSelfMoved :type Boolean) (HitLocation :type Vector :default "0, 0, 0") (HitNormal :type Vector :default "0, 0, 0") (NormalImpulse :type Vector :default "0, 0, 0") (Hit :type Hit%20Result%20Structure%20%28by%20ref%29))
  (Actor|DestroyActor))

(fn ConstructionScript)