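; BP_FinalGem is the final gem actor, animated as a hovering, spinning relic.
; BeginPlay records the mesh's relative start location.
; Each Tick yaws the gem at a set rate and moves it vertically in world space, flipping the bob speed whenever its relative height passes the offset limit above or below the start.
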(event EventBeginPlay
  (Variables|Default|SetStartPosition (Variables|/Script/Engine.SceneComponent|GetRelativeLocation (Variables|Default|GetSM_Gem))))

(event EventTick
  (params (DeltaSeconds :type Float%20%28single-precision%29))
  (bind _startposition (Variables|Default|GetStartPosition))
  (bind _sm_gem (Variables|Default|GetSM_Gem))
  (bind _offsetmax (Variables|Default|GetOffsetMax))
  (bind _relativelocation (Variables|/Script/Engine.SceneComponent|GetRelativeLocation _sm_gem))
  ;[1 1 1] Relic Hover / Rotation Animation
  (Utilities|FlowControl|Sequence
    (:then_0
      (Transformation|AddLocalRotation (Variables|Default|GetSM_Gem) (Math|Rotator|MakeRotator 0.0 0.0 (* (Variables|Default|GetRotationPerSecond) DeltaSeconds)) false false))
    (:then_1
      (Utilities|FlowControl|Sequence
        (:then_0
          (if (or (>= (.z _relativelocation) (+ (.z _startposition) _offsetmax)) (<= (.z _relativelocation) (- (.z _startposition) _offsetmax)))
            (Variables|Default|SetOffsetPerSecond (* (Variables|Default|GetOffsetPerSecond) -1.0))))
        (:then_1
          (Transformation|AddWorldOffset (Variables|Default|GetSM_Gem) (Math|Vector|MakeVector 0.0 0.0 (* DeltaSeconds (Variables|Default|GetOffsetPerSecond))) false false))))))

(fn ConstructionScript
  (|CallParentFunction))